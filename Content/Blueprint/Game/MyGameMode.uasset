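; Deathmatch game mode for a multiplayer FPS that tracks each player's name and score and runs a timed round.
; PostLogin starts character spawning and registers players in a controller-keyed map; the first join caches PlayerStarts and starts a one-second countdown.
; Rename, kill and self-death events rewrite map entries and push all values to every controller; self-death leaves score unchanged.
; Spawn requests cycle through PlayerStarts, and timer expiry signals game end to clients.
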(event Custom|RequestSpawn
  (params (PlayerController :type BP%20My%20Multi%20FPS%20Player%20Controller%20Object%20Reference))
  (Default|SpawnPlayerCharacter PlayerController "/Game/Blueprint/Player/BP_Attacker.BP_Attacker_C" (Transformation|GetActorTransform (Utilities|Array|Get(acopy) (Variables|Default|GetCharacterSpawnPoints) (Variables|Default|GetSpawnIndex))))
  (Variables|Default|SetSpawnIndex (+ (Variables|Default|GetSpawnIndex) 1))
  (if (>= (Variables|Default|GetSpawnIndex) (Utilities|Array|Length (Variables|Default|GetCharacterSpawnPoints)))
    (Variables|Default|SetSpawnIndex 0)))

(event Custom|UpdateValues
  (bind _keys (Utilities|Map|Keys (Variables|Default|GetPlayerGameDataMap)))
  (for _array_element _keys
    (bind _values (Utilities|Map|Values (Variables|Default|GetPlayerGameDataMap)))
    (Default|UpdateValues _array_element _values)))

(event Custom|ReName
  (params (PlayerController :type BP%20My%20Multi%20FPS%20Player%20Controller%20Object%20Reference) (NewName :type Name))
  (bind _playergamedatamap (Variables|Default|GetPlayerGameDataMap))
  (Variables|Default|SetTempScore (.PlayerScore (Utilities|Struct|BreakDeathMatchPlayerData (.Value (Utilities|Map|Find (Variables|Default|GetPlayerGameDataMap) PlayerController)))))
  (Utilities|Map|Remove _playergamedatamap PlayerController)
  (Utilities|Map|Add _playergamedatamap PlayerController (Utilities|Struct|MakeDeathMatchPlayerData NewName (Variables|Default|GetTempScore)))
  (CallFunction|UpdateValues))

(event Custom|KillAnother
  (params (PlayerController :type BP%20My%20Multi%20FPS%20Player%20Controller%20Object%20Reference))
  (bind _playergamedatamap (Variables|Default|GetPlayerGameDataMap))
  (bind _value (Utilities|Map|Find _playergamedatamap PlayerController))
  (bind (_playername _playerscore) (Utilities|Struct|BreakDeathMatchPlayerData _value))
  (Variables|Default|SetKillPlayerShortName _playername)
  (Variables|Default|SetKillPlayerShortScore (+ _playerscore 1))
  (Utilities|Map|Remove (Variables|Default|GetPlayerGameDataMap) PlayerController)
  (Utilities|Map|Add (Variables|Default|GetPlayerGameDataMap) PlayerController (Utilities|Struct|MakeDeathMatchPlayerData (Variables|Default|GetKillPlayerShortName) (Variables|Default|GetKillPlayerShortScore)))
  (CallFunction|UpdateValues))

(event Custom|SelfDeath
  (params (PlayerController :type BP%20My%20Multi%20FPS%20Player%20Controller%20Object%20Reference))
  (bind _playergamedatamap (Variables|Default|GetPlayerGameDataMap))
  (bind _value (Utilities|Map|Find _playergamedatamap PlayerController))
  (bind (_playername _playerscore) (Utilities|Struct|BreakDeathMatchPlayerData _value))
  (Variables|Default|SetHurtPlayerShortName _playername)
  (Variables|Default|SetHurtPlayerShortScore (- _playerscore 0))
  (Utilities|Map|Remove (Variables|Default|GetPlayerGameDataMap) PlayerController)
  (Utilities|Map|Add (Variables|Default|GetPlayerGameDataMap) PlayerController (Utilities|Struct|MakeDeathMatchPlayerData (Variables|Default|GetHurtPlayerShortName) (Variables|Default|GetHurtPlayerShortScore)))
  (CallFunction|UpdateValues))

(event Custom|GameStateSet
  (bind _outactors (Actor|GetAllActorsOfClass "/Script/Engine.PlayerStart"))
  (Variables|Default|SetCharacterSpawnPoints _outactors)
  (bind _returnvalue (Utilities|Time|SetTimerbyEvent (delegate Custom|Down) 1.0 true))
  (Variables|Default|SetDownTimerHandle _returnvalue))

(event Custom|Down
  (Variables|Default|SetRoundTime (- (Variables|Default|GetRoundTime) 1))
  (bind _keys (Utilities|Map|Keys (Variables|Default|GetPlayerGameDataMap)))
  (for _array_element _keys
    (Default|ClientUpdateDownTime _array_element (Variables|Default|GetRoundTime)))
  (if (<= (Variables|Default|GetRoundTime) 0)
    (Utilities|Time|ClearandInvalidateTimerbyHandle (Variables|Default|GetDownTimerHandle))
    (CallFunction|EndGame)))

(event Custom|EndGame
  (bind _keys (Utilities|Map|Keys (Variables|Default|GetPlayerGameDataMap)))
  (for _array_element _keys
    (Default|ClientEndGame _array_element)))

(event EventPostLogin
  (params (NewPlayer :type Player%20Controller%20Object%20Reference))
  (if (Variables|Default|GetFirstCharacterJoin)
    _
    (else
      (CallFunction|GameStateSet)
      (Variables|Default|SetFirstCharacterJoin true)))
  (bind _asbp_my_multi_fpsplayer_controller (Utilities|Casting|CastToBP_MyMultiFPSPlayerController NewPlayer))
  (Default|StartSpawnCharacter _asbp_my_multi_fpsplayer_controller)
  (Utilities|Map|Add (Variables|Default|GetPlayerGameDataMap) _asbp_my_multi_fpsplayer_controller (Utilities|Struct|MakeDeathMatchPlayerData (Utilities|String|StringToName (Utilities|GetObjectName _asbp_my_multi_fpsplayer_controller)))))

(fn ConstructionScript)