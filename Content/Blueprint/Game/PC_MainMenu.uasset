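; Player controller for the main menu that moves from an opening screen to the menu UI.
; On BeginPlay it creates the W_Main widget, adds it to the viewport and shows the mouse cursor.
; Pressing Space Bar removes that widget, creates and displays W_MainMenuUI, then switches input to UI-only without locking the mouse.
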(event EventBeginPlay
  (bind _returnvalue (UserInterface|CreateWidget "/Game/Blueprint/GameUI/W_Main.W_Main_C" self))
  (bind _output_get (Variables|Default|SetMain _returnvalue))
  (Utilities|IsValid _output_get
    (:Is%20Valid
      (UserInterface|Viewport|AddtoViewport _output_get 0)
      (Variables|Default|SetbShowMouseCursor true))))

(event Input|KeyboardEvents|SpaceBar
  (params (Key :type Key%20Structure :default "None"))
  (:Pressed
    (Widget|RemovefromParent (Variables|Default|GetMain))
    (bind _returnvalue (UserInterface|CreateWidget "/Game/Blueprint/GameUI/W_MainMenuUI.W_MainMenuUI_C" self))
    (bind _output_get (Variables|Default|SetMainMenu _returnvalue))
    (UserInterface|Viewport|AddtoViewport _output_get 0)
    (Input|SetInputModeUIOnly self 0 "DoNotLock")))

(fn ConstructionScript)