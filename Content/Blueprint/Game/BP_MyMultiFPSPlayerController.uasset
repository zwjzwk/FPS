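; Player controller for a multiplayer FPS deathmatch, linking the game mode to each player's pawn and UI.
; On death it reports the death and kill to MyGameMode, disables input, shows a timed death screen, then destroys the pawn and requests a respawn.
; It also spawns and possesses characters, toggles mouse input, relays renames and score updates, drives the HUD and shows end-game results before loading the main menu.
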(event Custom|SpawnPlayerCharacter
  (params (Class :type FPS%20Teach%20Base%20Character%20Class%20Reference) (SpawnTransform :type Transform))
  (bind _returnvalue (Game|SpawnActorfromClass Class SpawnTransform "Undefined" 0 0))
  (Pawn|Possess _returnvalue)
  (CallFunction|ClientHideMouse))

(event Custom|StartSpawnCharacter
  (Utilities|FlowControl|Delay 1.0)
  (bind _asmy_game_mode (Utilities|Casting|CastToMyGameMode (Game|GetGameMode)))
  (Default|RequestSpawn _asmy_game_mode self))

(event Custom|DeathUI
  (bind _returnvalue (UserInterface|CreateWidget "/Game/Blueprint/GameUI/W_DeathUI.W_DeathUI_C" self))
  (Utilities|IsValid _returnvalue
    (:Is%20Valid
      (UserInterface|Viewport|AddtoViewport _returnvalue 0)
      (Utilities|FlowControl|Delay (Variables|Default|GetDeathTime))
      (Widget|RemovefromParent _returnvalue))))

(event Custom|UpdateValues
  (params (Values :type Array%20of%20Death%20Match%20Player%20Data%20Structures))
  (bind _output_get (Variables|Default|SetValues Values))
  (Class|KismetMultiFPSLibrary|SortValues _output_get)
  (bind _playerui (Variables|Default|GetPlayerUI)
    (:then
      (Default|UpdateSortBox _playerui (Variables|Default|GetValues)))
    (:else)))

(event Custom|ServerRequireUpdateValues
  (bind _asmy_game_mode (Utilities|Casting|CastToMyGameMode (Game|GetGameMode)))
  (Default|UpdateValues _asmy_game_mode))

(event Custom|ClientDisableInput
  (Input|DisableInput (Pawn|GetControlledPawn) self))

(event Custom|ClientUpdateDownTime
  (params (DownTime :type Integer))
  (Variables|Default|SetDownTime DownTime))

(event Custom|ClientEndGame
  (params (Score :type Integer) (Death :type Integer))
  (bind _returnvalue (UserInterface|CreateWidget "/Game/Blueprint/GameUI/W_ClientEndGame.W_ClientEndGame_C" self))
  (Default|SetScore _returnvalue Score Death)
  (UserInterface|Viewport|AddtoViewport _returnvalue 0)
  (Utilities|FlowControl|Delay 3.0)
  (Game|OpenLevel(byName) "MainMenu"))

(event Custom|ClientHideMouse
  (Input|SetInputModeGameOnly self)
  (Variables|Default|SetbShowMouseCursor false))

(event Custom|SetPlayerName
  (params (NewName :type Text))
  (bind _asmy_game_mode (Utilities|Casting|CastToMyGameMode (Game|GetGameMode)))
  (Default|ReName _asmy_game_mode self (Utilities|String|StringToName (Utilities|String|ToString(Text) NewName))))

(event Custom|ClientShowMouse
  (Input|SetInputModeUIOnly self 0 "DoNotLock")
  (Variables|Default|SetbShowMouseCursor true))

(event EventDoCrosshairRecoil
  ;[1 1 1] UI
  (Default|DoCrosshairRecoil (Variables|Default|GetPlayerUI)))

(event EventUpdateAmmoUI
  (params (ClipCurrentAmmo :type Integer) (GunCurrentAmmo :type Integer))
  ;[1 1 1] UI
  (Default|UpdateAmmo (Variables|Default|GetPlayerUI) ClipCurrentAmmo GunCurrentAmmo))

(event EventCreatePlayerUI
  ;[1 1 1] UI
  (Variables|Default|GetPlayerUI
    (:then
      (Widget|RemovefromParent (Variables|Default|GetPlayerUI))
      (if (Pawn|IsLocalPlayerController)
        (bind _returnvalue (UserInterface|CreateWidget "/Game/Blueprint/GameUI/W_PlayerUI.W_PlayerUI_C" self))
        (bind _output_get (Variables|Default|SetPlayerUI _returnvalue))
        (UserInterface|Viewport|AddtoViewport _output_get 0)
        (CallFunction|ServerRequireUpdateValues)))
    (:else
      (if (Pawn|IsLocalPlayerController)
        (bind _returnvalue_2 (UserInterface|CreateWidget "/Game/Blueprint/GameUI/W_PlayerUI.W_PlayerUI_C" self))
        (bind _output_get_2 (Variables|Default|SetPlayerUI _returnvalue_2))
        (UserInterface|Viewport|AddtoViewport _output_get_2 0)
        (CallFunction|ServerRequireUpdateValues)))))

(event EventUpdateHealthUI
  (params (NewHealth :type Float%20%28single-precision%29))
  ;[1 1 1] UI
  (Default|UpdateHealth (Variables|Default|GetPlayerUI) NewHealth))

(event EventSetPlayerUIHidden
  (params (IsHidden :type Boolean))
  (bind _playerui (Variables|Default|GetPlayerUI))
  ;[1 1 1] UI
  (Utilities|IsValid _playerui
    (:Is%20Valid
      (if IsHidden
        (Widget|SetVisibility _playerui "Hidden")
        (else
          (Widget|SetVisibility _playerui "Visible"))))))

(event EventDeathMatchDeath
  (params (DamageActor :type Actor%20Object%20Reference))
  (bind _asmy_game_mode (Utilities|Casting|CastToMyGameMode (Game|GetGameMode)))
  (Default|SelfDeath _asmy_game_mode self)
  (CallFunction|ClientDisableInput)
  (bind _asbp_my_multi_fpsplayer_controller (Utilities|Casting|CastToBP_MyMultiFPSPlayerController (Game|GetInstigatorController DamageActor)))
  (Default|KillAnother _asmy_game_mode _asbp_my_multi_fpsplayer_controller)
  (CallFunction|DeathUI)
  (Utilities|FlowControl|Delay (Variables|Default|GetDeathTime))
  (Actor|DestroyActor (Pawn|GetControlledPawn))
  (bind _asmy_game_mode_2 (Utilities|Casting|CastToMyGameMode (Game|GetGameMode)))
  (Default|RequestSpawn _asmy_game_mode_2 self))

(event Input|KeyboardEvents|LeftAlt
  (params (Key :type Key%20Structure :default "None"))
  (:Pressed
    (CallFunction|ClientShowMouse)))

(fn ConstructionScript)