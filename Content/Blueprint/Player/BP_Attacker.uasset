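; Player Blueprint for the attacker, handling first-person arms pose updates, aim offsets and third-person body death.
; Blend pose changes are forwarded to the client arms AnimBP, while Tick derives Pitch and Yaw from aim versus actor rotation.
; Death chains through ServerPlay to MultiPlay, which plays a death animation on the mesh, then switches it to physics ragdoll after a short delay.
; Death UI widget creation is present but unconnected.
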(event Custom|ServerPlay
  (CallFunction|MultiPlay))

(event Custom|MultiPlay
  (bind _mesh (Variables|Character|GetMesh))
  (Components|Animation|PlayAnimation (Variables|Character|GetMesh) "/Game/Asset/TPBodysAnimation/Animation/Death_1.Death_1" false)
  (Utilities|FlowControl|Delay 0.95)
  (Physics|SetSimulatePhysics _mesh true)
  (Collision|SetCollisionEnabled _mesh "QueryAndPhysics"))

(event EventTPBodysDeath
  (CallFunction|ServerPlay))

(event EventTick
  (params (DeltaSeconds :type Float%20%28single-precision%29))
  (bind _returnvalue (Pawn|GetBaseAimRotation))
  (bind _returnvalue_2 (Transformation|GetActorRotation))
  (bind _returnvalue_3 (Math|Rotator|Delta(Rotator) _returnvalue _returnvalue_2))
  (Variables|Default|SetPitch (.pitch _returnvalue_3))
  (Variables|Default|SetYaw (.yaw _returnvalue_3)))

(event EventUpdateFPArmsBlendPose
  (params (NewIndex :type Integer))
  (Class|INTUpdateAnimBlendPose|UpdateBlendPose(Message) (Variables|Default|GetClientArmsAnimBP) NewIndex))

(fn ConstructionScript)